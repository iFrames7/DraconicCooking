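; Player character Blueprint that moves, grabs or drops objects and interacts with objects in front of it.
; A short forward sphere trace on separate channels finds targets, which receive grab or interact messages; grabbing with no target drops the held object.
; Grab attaches the object to the Hands component.
; SetIsInteracting stores the active object and toggles an interaction input mapping context, while stop input forwards to that object.
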(event `EnhancedInput|/Game/Miguel/Inputs/IA_Movement`
  (params (ActionValue :type "Vector2D Structure") (ElapsedSeconds :type "Float (double-precision)") (TriggeredSeconds :type "Float (double-precision)") (InputAction :type "InputAction Object Reference" :default "/Game/Miguel/Inputs/IA_Movement.IA_Movement"))
  (:`Triggered`
    (`self.AddMovementInput` (`KismetMathLibrary.Conv_Vector2DToVector` ActionValue))))

(event `EnhancedInput|/Game/Miguel/Inputs/IA_GrabDrop`
  (params (ActionValue :type Boolean) (ElapsedSeconds :type "Float (double-precision)") (TriggeredSeconds :type "Float (double-precision)") (InputAction :type "InputAction Object Reference" :default "/Game/Miguel/Inputs/IA_GrabDrop.IA_GrabDrop"))
  (bind (_returnvalue _grabbedobject) (`self.GetGrabbedObject`))
  (:`Started`
    (bind (_returnvalue_2 _outhit) (`self.Find Object to Interact With` "TraceTypeQuery3"))
    (if _returnvalue_2
      (message `/Game/Miguel/Blueprints/Interfaces/BPI_Interactable.Grab/Drop` (`.HitActor` (`GameplayStatics.BreakHitResult` _outhit)) self)
      (elif _returnvalue
        (`/Game/Miguel/Blueprints/Interactable/BP_Grabbable.Drop` _grabbedobject)
        (set `self.GrabbedObject` null)))))

(event `Grab`
  (params (ObjectToGrab :type "/Game/Miguel/Blueprints/Interactable/BP_Grabbable Object Reference"))
  (bind _output_get (set `self.GrabbedObject` ObjectToGrab))
  (`self.K2_AttachToComponent` _output_get (`self.Hands`) "None" "KeepWorld" "KeepWorld" "KeepWorld" true)
  (`KismetSystemLibrary.MoveComponentTo` (`Actor.RootComponent` (`self.GrabbedObject`))))

(event `EnhancedInput|/Game/Miguel/Inputs/IA_StartInteraction`
  (params (ActionValue :type Boolean) (ElapsedSeconds :type "Float (double-precision)") (TriggeredSeconds :type "Float (double-precision)") (InputAction :type "InputAction Object Reference" :default "/Game/Miguel/Inputs/IA_StartInteraction.IA_StartInteraction"))
  ;[0 1 0] StartInteraction
  (:`Started`
    (if (`self.IsInteracting`)
      (`self.StopInteraction`)
      (else
        (bind (_returnvalue _outhit) (`self.Find Object to Interact With` "TraceTypeQuery4"))
        (if _returnvalue
          (message `/Game/Miguel/Blueprints/Interfaces/BPI_Interactable.Interact` (`.HitActor` (`GameplayStatics.BreakHitResult` _outhit)) self))))))

(event `SetIsInteracting`
  (params (IsInteracting :type Boolean) (InteractingObject :type "/Game/Miguel/Blueprints/Interfaces/BPI_Interactable Interface"))
  (bind _returnvalue (pcsubsystem `EnhancedInputLocalPlayerSubsystem` (`GameplayStatics.GetPlayerController` 0)))
  ;[1 1 0] Set Is Interacting
  (set `self.IsInteracting` IsInteracting)
  (set `self.Interacting Object` InteractingObject)
  (if (`self.IsInteracting`)
    (`EnhancedInputSubsystemInterface.AddMappingContext` _returnvalue "/Game/Miguel/Inputs/IMC_Interaction.IMC_Interaction" 0 (struct))
    (else
      (`EnhancedInputSubsystemInterface.RemoveMappingContext` _returnvalue "/Game/Miguel/Inputs/IMC_Interaction.IMC_Interaction" (struct)))))

(event `EnhancedInput|/Game/Miguel/Inputs/IA_StopInteraction`
  (params (ActionValue :type Boolean) (ElapsedSeconds :type "Float (double-precision)") (TriggeredSeconds :type "Float (double-precision)") (InputAction :type "InputAction Object Reference" :default "/Game/Miguel/Inputs/IA_StopInteraction.IA_StopInteraction"))
  ;[1 0.4626 0] Stop Interaction
  (:`Started`
    (`self.StopInteraction`)))

(event `StopInteraction`
  ;[1 0.4626 0] Stop Interaction
  (`/Game/Miguel/Blueprints/Interfaces/BPI_Interactable.StopInteraction` (`self.Interacting Object`)))

(fn `Find Object to Interact With`
  (params (TraceChannel :type "ETraceTypeQuery Enum" :default "TraceTypeQuery1"))
  (returns (ReturnValue :type Boolean) (OutHit :type "HitResult Structure"))
  (bind _x (.x (+ (* (`self.GetActorForwardVector`) 50.0) (`self.K2_GetActorLocation`))))
  (bind _y (.y (+ (* (`self.GetActorForwardVector`) 50.0) (`self.K2_GetActorLocation`))))
  (bind _z (.z (+ (* (`self.GetActorForwardVector`) 50.0) (`self.K2_GetActorLocation`))))
  (bind (_outhit _returnvalue) (`KismetSystemLibrary.SphereTraceSingle` (`KismetMathLibrary.MakeVector` _x _y (+ _z -50.0)) (`KismetMathLibrary.MakeVector` _x _y (+ _z 10.0)) 30.0 TraceChannel false (`|MakeArray` (`self.GrabbedObject`) :!type "Actor Object Reference") "ForDuration"))
  (return _returnvalue _outhit))

(fn `GetGrabbedObject`
  (returns (ReturnValue :type Boolean) (GrabbedObject :type "/Game/Miguel/Blueprints/Interactable/BP_Grabbable Object Reference"))
  (bind _grabbedobject (`self.GrabbedObject`))
  (return (`KismetSystemLibrary.IsValid` _grabbedobject) _grabbedobject))

(fn `UserConstructionScript`)