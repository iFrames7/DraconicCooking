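; BP_OrderPickupArea is an interactable delivery spot where the player hands in filled plates to score points.
; On Grab/Drop it destroys a held non-empty BP_Plate, returns a plate to a plate box and increments Puntos.
; The target box is the connected one if valid, otherwise a random BP_PlateBox gathered on BeginPlay.
; Reaching the score target shows WBP_Win, switches to UI-only input and pauses the game.
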(event `self.ReceiveBeginPlay`
  (`self.ConnetedPlateBox`
    (:`then`)
    (:`else`
      (bind _outactors (`GameplayStatics.GetAllActorsOfClass` "/Game/Miguel/Blueprints/Interactable/BP_PlateBox.BP_PlateBox_C"))
      (set `self.AllPlateBoxes` _outactors))))

(event `/Game/Miguel/Blueprints/Interfaces/BPI_Interactable.Grab/Drop`
  (params (Player :type "/Game/Miguel/Blueprints/BP_Character Object Reference"))
  (bind _returnvalue (`GameplayStatics.GetPlayerController` 0))
  (bind _asbp_plate (cast `/Game/Miguel/Blueprints/Interactable/BP_Plate` (`.GrabbedObject` (`/Game/Miguel/Blueprints/BP_Character.GetGrabbedObject` Player))))
  (if (not (`/Game/Miguel/Blueprints/Interactable/BP_Kitchenware.IsEmpty` _asbp_plate))
    (`self.K2_DestroyActor` _asbp_plate)
    (set `/Game/Miguel/Blueprints/BP_Character.GrabbedObject` null Player)
    (`/Game/Miguel/Blueprints/Interactable/BP_PlateBox.AddPlate` (`self.GetCurrentPlateBox`))
    (bind _result (`/Engine/EditorBlueprintResources/StandardMacros.IncrementInt` (`self.Puntos`))
      (:`  `
        (set `self.Puntos` _result)
        (if (== (`self.Puntos`) 5)
          (bind _returnvalue_2 (`|CreateWidget` "/Game/WBP_Win.WBP_Win_C"))
          (`UserWidget.AddToViewport` _returnvalue_2 0)
          (set `PlayerController.bShowMouseCursor` true _returnvalue)
          (`WidgetBlueprintLibrary.SetInputMode_UIOnlyEx` _returnvalue null)
          (`GameplayStatics.SetGamePaused` true))))))

(fn `GetCurrentPlateBox`
  (returns (ConnetedPlateBox :type "/Game/Miguel/Blueprints/Interactable/BP_PlateBox Object Reference"))
  (bind _connetedplatebox (`self.ConnetedPlateBox`)
    (:`then`
      (return _connetedplatebox))
    (:`else`
      (return (`KismetArrayLibrary.Array_Random` (`self.AllPlateBoxes`))))))

(fn `UserConstructionScript`)