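; BP_PlateBox is an interactable box that dispenses BP_Plate actors from a stack.
; On BeginPlay, InitPlates spawns the default number of plates above ObjectPlace, removes their physics and attaches them, using that same count as the vertical spacing multiplier.
; Grab/Drop checks whether the last plate can be grabbed, then passes it to the player and removes it from the array.
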(event `self.ReceiveBeginPlay`
  (`self.InitPlates`))

(event `/Game/Miguel/Blueprints/Interfaces/BPI_Interactable.Grab/Drop`
  (params (Player :type "/Game/Miguel/Blueprints/BP_Character Object Reference"))
  (bind _plate (`self.plate`))
  (if (`KismetArrayLibrary.Array_IsNotEmpty` (`self.plate`))
    (if (`/Game/Miguel/Blueprints/Interactable/BP_Grabbable.canBeGrabbed` (`|GetArrayItem` _plate (`KismetArrayLibrary.Array_LastIndex` _plate)) Player)
      (`self.Grab` Player))))

(event `self.Grab`
  (params (player :type "/Game/Miguel/Blueprints/BP_Character Object Reference"))
  (bind _plate (`self.plate`))
  (bind _output (`|GetArrayItem` _plate (`KismetArrayLibrary.Array_LastIndex` _plate)))
  (`/Game/Miguel/Blueprints/Interactable/BP_Grabbable.Grab` _output player)
  (`KismetArrayLibrary.Array_RemoveItem` (`self.plate`) _output))

(fn `InitPlates`
  (bind (_returnvalue_x _returnvalue_y _returnvalue_z) (`KismetMathLibrary.BreakVector` (`SceneComponent.K2_GetComponentLocation` (`self.ObjectPlace`))))
  (for _index (range 1 (+ (`self.defaultPlatesAmount`) 1))
    (bind _returnvalue (`|SpawnActorFromClass` "/Game/Miguel/Blueprints/Interactable/BP_Plate.BP_Plate_C" (`KismetMathLibrary.MakeTransform` (`KismetMathLibrary.MakeVector` _returnvalue_x _returnvalue_y (+ _returnvalue_z (* (- _index 1) (`self.defaultPlatesAmount`))))) "Undefined" "MultiplyWithRoot" null null))
    (`/Game/Miguel/Blueprints/Interactable/BP_Grabbable.RemovePhysics` _returnvalue)
    (`self.K2_AttachToComponent` _returnvalue (`self.ObjectPlace`) "None" "KeepWorld" "KeepWorld" "KeepWorld" true)
    (`KismetArrayLibrary.Array_Add` (`self.plate`) _returnvalue)))

(fn `UserConstructionScript`
  (`parent.UserConstructionScript`))