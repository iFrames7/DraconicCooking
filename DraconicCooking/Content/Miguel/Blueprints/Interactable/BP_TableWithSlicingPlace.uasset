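; Interactable table with a slicing place where a player slices a placed BP_FoodItem.
; Interact checks that the food can be sliced, changes its state and marks the player as interacting.
; Tick advances Progress at a constant rate, printing it on screen, then ends the interaction and sets the food's next state.
; Grab/drop only works at zero or full progress and resets it, so partly sliced food stays put.
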(event `self.ReceiveTick`
  (params (DeltaSeconds :type "Float (single-precision)"))
  (`parent.ReceiveTick` DeltaSeconds)
  (if (`self.isInteracting`)
    (bind _output_get (set `self.progress` (`KismetMathLibrary.FInterpTo_Constant` (`self.progress`) 1.0 DeltaSeconds (`self.slicingSpeed`))))
    (`KismetSystemLibrary.PrintString` (`KismetStringLibrary.Conv_DoubleToString` _output_get) true true (struct :`G` 0.66 :`B` 1.0 :`A` 1.0) DeltaSeconds)
    (if (== (`self.progress`) 1.0)
      (`/Game/Miguel/Blueprints/Interfaces/BPI_Interactable.StopInteraction`)
      (bind _asbp_food_item (cast `/Game/Miguel/Blueprints/Interactable/BP_FoodItem` (`self.PlacedObject`)))
      (`/Game/Miguel/Blueprints/Interactable/BP_FoodItem.SetState` _asbp_food_item "NewEnumerator2"))))

(event `/Game/Miguel/Blueprints/Interfaces/BPI_Interactable.Grab/Drop`
  (params (Player :type "/Game/Miguel/Blueprints/BP_Character Object Reference"))
  (if (`self.canGrabObject`)
    (`parent.Grab/Drop` Player)
    (set `self.progress` 0.0)))

(event `/Game/Miguel/Blueprints/Interfaces/BPI_Interactable.Interact`
  (params (player :type "/Game/Miguel/Blueprints/BP_Character Object Reference"))
  (bind _asbp_food_item (cast `/Game/Miguel/Blueprints/Interactable/BP_FoodItem` (`self.PlacedObject`)))
  (if (`/Game/Miguel/Blueprints/Interactable/BP_FoodItem.canBeSliced` _asbp_food_item)
    (`/Game/Miguel/Blueprints/Interactable/BP_FoodItem.SetState` _asbp_food_item "NewEnumerator1")
    (`/Game/Miguel/Blueprints/BP_Character.SetIsInteracting` player true self)
    (set `self.interactingPlayer` player)
    (set `self.isInteracting` true)))

(event `/Game/Miguel/Blueprints/Interfaces/BPI_Interactable.StopInteraction`
  (set `self.isInteracting` false)
  (`/Game/Miguel/Blueprints/BP_Character.SetIsInteracting` (`self.interactingPlayer`) false null))

(fn `canGrabObject`
  (returns (canGrabObject :type Boolean))
  (return (or (== (`self.progress`) 0.0) (== (`self.progress`) 1.0))))

(fn `UserConstructionScript`
  (`parent.UserConstructionScript`))