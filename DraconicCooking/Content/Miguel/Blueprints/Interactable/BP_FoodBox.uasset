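; BP_FoodBox is an interactable food crate that hands out a food item of its configured FoodItemAsset.
; Grab/Drop spawns a BP_FoodItem and gives it to the player when nothing is placed on the box and the player's hands are empty.
; It defers to parent grab/drop when the player holds something or the placed object can be grabbed.
; The construction script shows the asset's icon on the cube through a dynamic material.
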(event `/Game/Miguel/Blueprints/Interfaces/BPI_Interactable.Grab/Drop`
  (params (Player :type "/Game/Miguel/Blueprints/BP_Character Object Reference"))
  (bind _placedobject (`self.PlacedObject`)
    (:`then`
      (if (`/Game/Miguel/Blueprints/Interactable/BP_Grabbable.canBeGrabbed` _placedobject Player)
        (`parent.Grab/Drop` Player :!label _label)))
    (:`else`
      (if (`/Game/Miguel/Blueprints/BP_Character.GetGrabbedObject` Player)
        (goto _label)
        (else
          (bind _returnvalue (`|SpawnActorFromClass` "/Game/Miguel/Blueprints/Interactable/BP_FoodItem.BP_FoodItem_C" (`self.GetTransform`) "Undefined" "MultiplyWithRoot" null true (`self.FoodItemAsset`) null))
          (`/Game/Miguel/Blueprints/Interfaces/BPI_Interactable.Grab/Drop` _returnvalue Player))))))

(fn `UserConstructionScript`
  (`parent.UserConstructionScript`)
  (bind _returnvalue (`KismetMaterialLibrary.CreateDynamicMaterialInstance` "/Game/FoodModels/Materials/M_FoodBox.M_FoodBox"))
  (`MaterialInstanceDynamic.SetTextureParameterValue` _returnvalue "Icon" (`/Game/Miguel/Blueprints/AssetTypes/DA_FoodItemBP.Icon` (`self.FoodItemAsset`)))
  (`PrimitiveComponent.SetMaterial` (`self.Cube`) 0 _returnvalue))