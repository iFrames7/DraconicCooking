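; Cookware Blueprint that runs a timed cooking process on the items it holds.
; Cook switches cooking on or off and starts progress updates only when Items is not empty.
; UpdateCookingProgress re-calls itself after a short Delay instead of using Tick, raising and printing CookingScore each pass.
; Cooking stops once the score reaches the per-item target times the item count, so more items take longer.
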(event `/Game/Ricardo/BPI_Cookware.Cook`
  (params (enable :type Boolean))
  (bind _output_get (set `self.IsCooking` enable))
  (if (and _output_get (`KismetMathLibrary.Conv_IntToBool` (`KismetArrayLibrary.Array_Length` (`self.Items`))))
    (`self.UpdateCookingProgress`)))

(event `UpdateCookingProgress`
  (bind _result (`/Engine/EditorBlueprintResources/StandardMacros.IncrementInt` (`self.CookingScore`))
    (:`  `
      (`KismetSystemLibrary.PrintString` (`KismetStringLibrary.Conv_IntToString` _result))
      (`KismetSystemLibrary.Delay` 0.2)
      (if (>= (`self.CookingScore`) (* (`self.CookingTargetScorePerItem`) (`KismetArrayLibrary.Array_Length` (`self.Items`))))
        (set `self.IsCooking` false))
      (if (`self.IsCooking`)
        (`self.UpdateCookingProgress`)))))

(fn `UserConstructionScript`
  (`parent.UserConstructionScript`))